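; BP_Agent is an AI agent that wanders the navmesh and can be called over to a cart.
; On BeginPlay it loops a roam: move to a random nearby navigable point, wait briefly, then repeat, only while moves succeed.
; ComeToCart sends it to the given cart actor and snap-attaches it there on arrival.
; Roaming is never explicitly stopped, and failed moves have no handling.
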(event Custom|AIRoamAround
  (bind _randomlocation (Class|NavigationSystemV1|GetRandomLocationinNavigableRadius (Transformation|GetActorLocation) 2e+02 0 0))
  (AI|AIMoveTo self _randomlocation 0 5e+01 false
    (:OnSuccess
      (Utilities|FlowControl|Delay 2.0)
      (CallFunction|AIRoamAround)
      (Development|PrintString "Hello"))))

(event Custom|ComeToCart
  (params (Cart%20Actor :type Cart%20BP%20Object%20Reference))
  (AI|AIMoveTo self (Transformation|GetActorLocation Cart%20Actor) 0 1e+02 false
    (:OnSuccess
      (Transformation|AttachActorToActor Cart%20Actor "None" "SnapToTarget" "SnapToTarget" "KeepRelative" true)
      (Development|PrintString "attached"))))

(event EventBeginPlay
  (CallFunction|AIRoamAround))

(event Collision|EventActorBeginOverlap
  (params (OtherActor :type Actor%20Object%20Reference)))

(event EventTick
  (params (DeltaSeconds :type Float%20%28single-precision%29)))

(fn ConstructionScript)