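; Cart actor that rides along a spline from start to end when play begins.
; BeginPlay fires the MoveCart event, which plays the MovingCart timeline.
; Each update maps the timeline alpha to a distance along the SplineRef actor's spline, then sets the cart's world location and rotation to match that point.
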(event Custom|MoveCart
  (bind _spline_ref (Variables|Default|GetSpline_ref))
  (bind _spline (Variables|/Game/Spline_BP.Spline_BP_C|GetSpline _spline_ref))
  (bind _newtrack_1 (Timeline|MovingCart Play)
    (:Update
      (Variables|Default|SetBlend _newtrack_1)
      (Transformation|SetActorLocationAndRotation (Spline|GetLocationatDistanceAlongSpline _spline (Math|Float|Lerp 0.0 (Spline|GetSplineLength (Variables|/Game/Spline_BP.Spline_BP_C|GetSpline (Variables|Default|GetSpline_ref))) (Variables|Default|GetBlend)) "World") (Spline|GetRotationatDistanceAlongSpline _spline (Math|Float|Lerp 0.0 (Spline|GetSplineLength (Variables|/Game/Spline_BP.Spline_BP_C|GetSpline (Variables|Default|GetSpline_ref))) (Variables|Default|GetBlend)) "World")))))

(event EventBeginPlay
  (CallFunction|MoveCart))

(event Collision|EventActorBeginOverlap
  (params (OtherActor :type Actor%20Object%20Reference)))

(event EventTick
  (params (DeltaSeconds :type Float%20%28single-precision%29)))

(fn ConstructionScript)