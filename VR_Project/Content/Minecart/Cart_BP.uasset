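; Minecart actor that carries the VR player along spline paths and calls a BP_Agent to it on BeginPlay.
; Its Radius overlap toggles CartActive on the VRPawn; InputActive attaches the pawn at an offset and starts the ride.
; A timeline scaled by Speed drives position and rotation along CartPath's spline.
; On finishing, it switches to CartPath2 and restarts, so that second path repeats thereafter.
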(event OnComponentBeginOverlap(Radius)
  (params (OverlappedComponent :type Primitive%20Component%20Object%20Reference) (OtherActor :type Actor%20Object%20Reference) (OtherComp :type Primitive%20Component%20Object%20Reference) (OtherBodyIndex :type Integer) (bFromSweep :type Boolean) (SweepResult :type Hit%20Result%20Structure%20%28by%20ref%29))
  (bind _outactors (Actor|GetAllActorsOfClass "/Game/VRTemplate/Blueprints/VRPawn.VRPawn_C"))
  (Variables|/Game/VRTemplate/Blueprints/VRPawn.VRPawn_C|SetcartActive (Utilities|Array|Get(acopy) _outactors) true))

(event OnComponentEndOverlap(Radius)
  (params (OverlappedComponent :type Primitive%20Component%20Object%20Reference) (OtherActor :type Actor%20Object%20Reference) (OtherComp :type Primitive%20Component%20Object%20Reference) (OtherBodyIndex :type Integer))
  (bind _outactors (Actor|GetAllActorsOfClass "/Game/VRTemplate/Blueprints/VRPawn.VRPawn_C"))
  (Variables|/Game/VRTemplate/Blueprints/VRPawn.VRPawn_C|SetcartActive (Utilities|Array|Get(acopy) _outactors) false))

(event Custom|MoveCart
  (Components|Timeline|SetPlayRate (Variables|Default|GetMovingCart) (/ 1.0 (Variables|Default|GetSpeed)))
  (bind _newtrack_0 (Timeline|MovingCart PlayFromStart)
    (:Update
      (Variables|Default|SetBlend _newtrack_0)
      (Transformation|SetActorLocationAndRotation (Spline|GetLocationatDistanceAlongSpline (Variables|/Game/Test_Build_1/rail/BP_Path.BP_Path_C|GetSpline (Variables|Default|GetCart_Path)) (Math|Float|Lerp 0.0 (Spline|GetSplineLength (Variables|/Game/Test_Build_1/rail/BP_Path.BP_Path_C|GetSpline (Variables|Default|GetCart_Path))) (Variables|Default|GetBlend)) "World") (Spline|GetRotationatDistanceAlongSpline (Variables|/Game/Test_Build_1/rail/BP_Path.BP_Path_C|GetSpline (Variables|Default|GetCart_Path)) (Math|Float|Lerp 0.0 (Spline|GetSplineLength (Variables|/Game/Test_Build_1/rail/BP_Path.BP_Path_C|GetSpline (Variables|Default|GetCart_Path))) (Variables|Default|GetBlend)) "World")))
    (:Finished
      ;[0.15 0.15 0.15 0.5] This should be updated to handle as many paths as we need. Ideally though, we'll only be using 2 paths and just looping the enviornment
      (Development|PrintString "Moving to Spline 2")
      (Variables|Default|SetCart_Path (Variables|Default|GetCart_Path_2))
      (CallFunction|MoveCart))))

(event Custom|InputActive
  (bind _outactors (Actor|GetAllActorsOfClass "/Game/VRTemplate/Blueprints/VRPawn.VRPawn_C"))
  (Transformation|AttachActorToActor (Utilities|Array|Get(acopy) _outactors) self "None" "KeepRelative" "KeepRelative" "KeepRelative" true)
  (Transformation|SetActorLocation (Utilities|Array|Get(acopy) _outactors) "0, 0, 0" false false)
  (Transformation|AddActorLocalOffset (Utilities|Array|Get(acopy) _outactors) (Variables|Default|GetPlayerOffset) false false)
  (CallFunction|MoveCart))

(event Input|EnhancedActionEvents|EnhancedInputActionIA_Hand_IndexCurl_Left
  (params (ActionValue :type Float%20%28double-precision%29) (ElapsedSeconds :type Float%20%28double-precision%29) (TriggeredSeconds :type Float%20%28double-precision%29) (InputAction :type Input%20Action%20Object%20Reference :default "/Game/VRTemplate/Input/Actions/Hands/IA_Hand_IndexCurl_Left.IA_Hand_IndexCurl_Left")))

(event EventBeginPlay
  (bind _outactors (Actor|GetAllActorsOfClass "/Game/AI/BP_Agent.BP_Agent_C"))
  (bind _asbp_agent (Utilities|Casting|CastToBP_Agent (Utilities|Array|Get(acopy) _outactors)))
  (Default|CometoCart _asbp_agent self)
  (Development|PrintString "Hello"))

(event Collision|EventActorBeginOverlap
  (params (OtherActor :type Actor%20Object%20Reference)))

(event EventTick
  (params (DeltaSeconds :type Float%20%28single-precision%29))
  (if (Variables|Default|GetcanMove)
    _))

(fn ConstructionScript)